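; Photo camera mockup actor that captures to a render target and detects tagged animals and hunters in view.
; TakePhotoEvent checks actors overlapping a cone frustum, then briefly flashes a spotlight and shows confirmation text.
; Animals get visibility line traces whose blocking result is only printed as debug text.
; Hunters ("Cazador") spawn a report button positioned from the VR player's forward vector, without adding the player's location.
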(event `TakePhotoEvent`
  (bind _confimationtext (`self.ConfimationText`))
  (bind _spotlight (`self.SpotLight`))
  (`self.TakePhoto`)
  (`SceneComponent.SetVisibility` _spotlight true false)
  (`KismetSystemLibrary.Delay` 0.01)
  (`SceneComponent.SetVisibility` _spotlight false false)
  (`SceneComponent.SetVisibility` _confimationtext true false)
  (`KismetSystemLibrary.Delay` 1.0)
  (`SceneComponent.SetVisibility` _confimationtext false false))

(event `self.ReceiveBeginPlay`
  (`SceneComponent.SetVisibility` (`self.SpotLight`) false false)
  (`SceneComponent.SetVisibility` (`self.ConfimationText`) false false))

(event `self.conoFrustum.OnComponentBeginOverlap`
  (params (OverlappedComponent :type "PrimitiveComponent Object Reference") (OtherActor :type "Actor Object Reference") (OtherComp :type "PrimitiveComponent Object Reference") (OtherBodyIndex :type Integer) (bFromSweep :type Boolean) (SweepResult :type "HitResult Structure (by ref)")))

(fn `SpawnButton`
  (bind _asc_vrep (cast `/Game/Blueprints/Base/C_VREP` (`GameplayStatics.GetPlayerCharacter` 0)))
  (`|SpawnActorFromClass` "/Game/Blueprints/Mockup/BP_BotonDenunciar.BP_BotonDenunciar_C" (`KismetMathLibrary.MakeTransform` (+ (* (`SceneComponent.GetForwardVector` (`VRCharacter.VRRootReference` _asc_vrep)) 100.0) (0.0 0.0 120.0)) (struct :`Pitch` 40.0)) "Undefined" "OverrideRootScale" null null))

(fn `TakePhoto`
  (locals (PosiblePhotoActor :type "Array of Actor Object Reference"))
  (bind _posiblephotoactor (`local.PosiblePhotoActor`))
  (`KismetSystemLibrary.PrintString` "Taking photo...")
  (for (_array_element _array_index) (`PrimitiveComponent.GetOverlappingActors` (`self.conoFrustum`) null)
    (if (`self.ActorHasTag` _array_element "Animal")
      (`KismetArrayLibrary.Array_Set` _posiblephotoactor _array_index _array_element true)
      (for _array_element_2 _posiblephotoactor
        (`KismetSystemLibrary.PrintString` (`KismetStringLibrary.Concat_StrStr` "Detected animal: " (`KismetSystemLibrary.GetObjectName` _array_element_2)))
        (bind (_outhits _returnvalue) (`KismetSystemLibrary.LineTraceMulti` (`self.K2_GetActorLocation`) (`self.K2_GetActorLocation` _array_element_2) "TraceTypeQuery1" false (`local.PosiblePhotoActor`)))
        (`KismetSystemLibrary.PrintString` (`KismetStringLibrary.Concat_StrStr` "Something is blocking the photo?: " (`KismetStringLibrary.Conv_BoolToString` _returnvalue))))
      (elif (`self.ActorHasTag` _array_element "Cazador")
        (`KismetSystemLibrary.PrintString` "Hunter detected...")
        (`self.SpawnButton`)))))

(fn `UserConstructionScript`
  (set `SceneCaptureComponent2D.TextureTarget` (`self.CameraRenderTarget`) (`self.SceneCaptureComponent2D`)))