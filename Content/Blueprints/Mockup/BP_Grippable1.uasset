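; Grippable waste pickup for a sorting mechanic, where each item has a waste type (TipoDesecho) to match against a bin (BP_Caneca).
; On BeginPlay it tints a dynamic material and its point light by type.
; Gripping activates all BP_Canecas actors and plays a Wwise sound.
; Overlapping a bin plays a sound, destroys the item and prints whether it was correct, meaning inside InnerCollision with a matching type.
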(event `self.ReceiveBeginPlay`
  (`self.AsignarTipo`))

(event `VRGripInterface.OnGrip`
  (params (GrippingController :type "GripMotionControllerComponent Object Reference") (GripInformation :type "BPActorGripInformation Structure (by ref)"))
  (`self.SetCanecas` true)
  (`AkGameplayStatics.PostEventAtLocation` (`self.WwiseGripEvent`) (`self.K2_GetActorLocation`)))

(event `self.ReceiveActorBeginOverlap`
  (params (OtherActor :type "Actor Object Reference"))
  (bind _asbp_caneca (cast `/Game/Blueprints/Mockup/BP_Caneca` OtherActor))
  (`self.GestionarResiduo` (and (`PrimitiveComponent.IsOverlappingActor` (`/Game/Blueprints/Mockup/BP_Caneca.InnerCollision` _asbp_caneca) self) (`|EnumEquality` (`self.TipoDesecho`) (`/Game/Blueprints/Mockup/BP_Caneca.TipoCaneca` _asbp_caneca)))))

(fn `AsignarTipo`
  (bind _staticmeshcomponent (`self.StaticMeshComponent`))
  (bind _coloresportipo (`self.ColoresPorTipo`))
  (bind _pointlight (`self.PointLight`))
  (bind _returnvalue (`KismetMathLibrary.Conv_ColorToLinearColor` (`|GetArrayItem` _coloresportipo)))
  (bind _returnvalue_2 (`KismetMathLibrary.Conv_ColorToLinearColor` (`|GetArrayItem` _coloresportipo 1)))
  (bind _returnvalue_3 (`KismetMathLibrary.Conv_ColorToLinearColor` (`|GetArrayItem` _coloresportipo 2)))
  (switch `/Game/Blueprints/Mockup/EnumCaneca` (`self.TipoDesecho`)
    (:`NewEnumerator0`
      (bind _returnvalue_4 (`PrimitiveComponent.CreateDynamicMaterialInstance` _staticmeshcomponent 0 "/Game/Materials/MI_Pickups.MI_Pickups" "None"))
      (bind _output_get (set `self.TempMatInst` _returnvalue_4))
      (`MaterialInstanceDynamic.SetVectorParameterValue` _output_get "Albedo Tint" _returnvalue)
      (`LightComponent.SetLightColor` _pointlight _returnvalue true))
    (:`NewEnumerator1`
      (bind _returnvalue_5 (`PrimitiveComponent.CreateDynamicMaterialInstance` _staticmeshcomponent 0 null "None"))
      (bind _output_get_2 (set `self.TempMatInst` _returnvalue_5))
      (`MaterialInstanceDynamic.SetVectorParameterValue` _output_get_2 "Albedo Tint" _returnvalue_2)
      (`LightComponent.SetLightColor` _pointlight _returnvalue_2 true))
    (:`NewEnumerator2`
      (bind _returnvalue_6 (`PrimitiveComponent.CreateDynamicMaterialInstance` _staticmeshcomponent 0 null "None"))
      (bind _output_get_3 (set `self.TempMatInst` _returnvalue_6))
      (`MaterialInstanceDynamic.SetVectorParameterValue` _output_get_3 "Albedo Tint" _returnvalue_3)
      (`LightComponent.SetLightColor` _pointlight _returnvalue_3 true))))

(fn `GestionarResiduo`
  (params (EsResiduoCorrecto :type Boolean))
  (`|ExecutionSequence`
    (:`then_0`
      (`AkGameplayStatics.PostEventAtLocation` (`self.WwiseDestroyEvent`) (`self.K2_GetActorLocation`)))
    (:`then_1`
      (if EsResiduoCorrecto
        (`self.K2_DestroyActor` self)
        (`KismetSystemLibrary.PrintString` "Tipo de desecho correcto")
        (else
          (`self.K2_DestroyActor` self)
          (`KismetSystemLibrary.PrintString` "Tipo de desecho incorrecto"))))))

(fn `SetCanecas`
  (params (Activar :type Boolean))
  (`KismetSystemLibrary.PrintString` "Set Canecas")
  (bind _outactors (`GameplayStatics.GetAllActorsOfClass` "/Game/Blueprints/Mockup/BP_Canecas.BP_Canecas_C"))
  (for _array_element _outactors
    (bind _output_get (set `self.Canecas` _array_element))
    (`/Game/Blueprints/Mockup/BP_Canecas.SetActivacion` _output_get Activar)))

(fn `UserConstructionScript`)