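; BP_Canecas is an actor grouping three BP_Caneca bins as child actors, with three boards and a score text.
; SetActivacion acts only on a state change, passing the new state to each bin and matching the boards' visibility to it.
; The score text starts hidden, and ShowTimedPuntaje shows it briefly.
; StartTimedDeactivation is empty, and the timed auto-deactivation logic is disconnected.
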(event `StartTimedDeactivation`)

(event `self.ReceiveBeginPlay`
  (`self.ShowPuntaje` false))

(event `ShowTimedPuntaje`
  (`self.ShowPuntaje` true)
  (`KismetSystemLibrary.Delay` 2.0)
  (`self.ShowPuntaje` false))

(fn `SetActivacion`
  (params (Activado :type Boolean))
  (if (!= Activado (`self.EstaActivo`))
    (`|ExecutionSequence`
      (:`then_0`
        (bind _asbp_caneca (cast `/Game/Blueprints/Mockup/BP_Caneca` (`ChildActorComponent.ChildActor` (`self.Caneca1`))))
        (`/Game/Blueprints/Mockup/BP_Caneca.SetActivado` _asbp_caneca Activado))
      (:`then_1`
        (bind _asbp_caneca_2 (cast `/Game/Blueprints/Mockup/BP_Caneca` (`ChildActorComponent.ChildActor` (`self.Caneca2`))))
        (`/Game/Blueprints/Mockup/BP_Caneca.SetActivado` _asbp_caneca_2 Activado))
      (:`then_2`
        (bind _asbp_caneca_3 (cast `/Game/Blueprints/Mockup/BP_Caneca` (`ChildActorComponent.ChildActor` (`self.Caneca3`))))
        (`/Game/Blueprints/Mockup/BP_Caneca.SetActivado` _asbp_caneca_3 Activado)))
    (set `self.EstaActivo` Activado)
    (`|ExecutionSequence`
      (:`then_0`
        (`SceneComponent.SetVisibility` (`self.Tablero2`) Activado false))
      (:`then_1`
        (`SceneComponent.SetVisibility` (`self.Tablero3`) Activado false))
      (:`then_2`
        (`SceneComponent.SetVisibility` (`self.Tablero1`) Activado false)))))

(fn `ShowPuntaje`
  (params (Show :type Boolean))
  (`SceneComponent.SetVisibility` (`self.TextRender`) Show false))

(fn `UserConstructionScript`)