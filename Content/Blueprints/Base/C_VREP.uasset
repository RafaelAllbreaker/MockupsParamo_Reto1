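; C_VREP is a VR Blueprint that grips and drops objects with the left and right motion controller triggers through VR Expansion Plugin interface calls.
; Trigger presses call TryGrip, which line-traces briefly forward and grips the hit component unless it denies gripping.
; Releases call LeaveGrip, which drops all that controller's grips.
; Both hands share GrippedObject, TryGrip updates only CanGripL, and GetControllerHand's name check is unconnected.
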(event `Key|MotionController_Left_Trigger`
  (params (Key :type "Key Structure"))
  (bind _leftmotioncontroller (`self.LeftMotionController`))
  (:`Pressed`
    (`self.TryGrip` _leftmotioncontroller))
  (:`Released`
    (`self.LeaveGrip` _leftmotioncontroller)))

(event `Key|MotionController_Right_Trigger`
  (params (Key :type "Key Structure"))
  (bind _rightmotioncontroller (`self.RightMotionController`))
  (:`Pressed`
    (`self.TryGrip` _rightmotioncontroller))
  (:`Released`
    (`self.LeaveGrip` _rightmotioncontroller)))

(fn `LeaveGrip`
  (params (MotionController :type "GripMotionControllerComponent Object Reference"))
  (for _array_element (`GripMotionControllerComponent.GetAllGrips` MotionController)
    (bind _returnvalue (`GripMotionControllerComponent.DropObjectByInterface` MotionController (`self.GrippedObject`) (`.GripID` (break `BPActorGripInformation` _array_element)) (0.0 0.0 0.0) (0.0 0.0 0.0)))
    (if (`self.GetControllerHand` MotionController)
      (set `self.CanGripL` _returnvalue)
      (else
        (set `self.CanGripR` _returnvalue)))
    (set `self.GrippedObject` null)))

(fn `TryGrip`
  (params (MotionController :type "GripMotionControllerComponent Object Reference"))
  (bind _returnvalue (`SceneComponent.K2_GetComponentLocation` MotionController))
  (if (`self.GetControllerHand` MotionController)
    (if (`self.CanGripL`)
      (bind (_outhit _returnvalue_2) (`KismetSystemLibrary.LineTraceSingle` _returnvalue (+ _returnvalue (* (`SceneComponent.GetForwardVector` MotionController) 10.0)) "TraceTypeQuery1" true :!label _label))
      (if _returnvalue_2
        (bind _output_get (set `self.GrippedObject` (`.HitComponent` (`GameplayStatics.BreakHitResult` _outhit))))
        (bind _returnvalue_3 (message `VRGripInterface.DenyGripping` _output_get))
        (if (not _returnvalue_3)
          (bind _returnvalue_4 (`GripMotionControllerComponent.GripObjectByInterface` MotionController _output_get (`SceneComponent.K2_GetComponentToWorld` _output_get) false "None" false))
          (set `self.CanGripL` (not _returnvalue_4)))))
    (elif (`self.CanGripR`)
      (goto _label))))

(fn `UserConstructionScript`)